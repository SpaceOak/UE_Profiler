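; StaticCameraProfiling is an actor that cycles the player's view through the CameraActors placed in the level, apparently for profiling from fixed viewpoints.
; On BeginPlay it gathers all CameraActors, enables input from the first player controller and blends the view to the camera at the current index.
; A Space bar debug key advances the index with wraparound and blends to the next camera.
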(event EventBeginPlay
  (bind _outactors (Actor|GetAllActorsOfClass "/Script/Engine.CameraActor"))
  (Variables|Default|SetOut%20Actors _outactors)
  (Input|EnableInput (Game|GetPlayerController 0))
  (Game|Player|SetViewTargetwithBlend (Game|GetPlayerController 0) (Utilities|Array|Get(acopy) (Variables|Default|GetOut%20Actors) (Variables|Default|GetCameraIdx)) 1.0 "VTBlend_Linear" 0.0 false))

(event Collision|EventActorBeginOverlap
  (params (OtherActor :type Actor%20Object%20Reference)))

(event EventTick
  (params (DeltaSeconds :type Float%20%28single-precision%29)))

(event Input|KeyboardEvents|DebugKeySpaceBar
  (params (Key :type Key%20Structure) (ActionValue :type Input%20Action%20Value%20Structure))
  (:Pressed
    (Variables|Default|SetCameraIdx (Math|Integer|%(Integer) (+ (Variables|Default|GetCameraIdx) 1) (Utilities|Array|Length (Variables|Default|GetOut%20Actors))))
    (Game|Player|SetViewTargetwithBlend (Game|GetPlayerController 0) (Utilities|Array|Get(acopy) (Variables|Default|GetOut%20Actors) (Variables|Default|GetCameraIdx)) 1.0 "VTBlend_Linear" 0.0 false)))

(fn ConstructionScript)